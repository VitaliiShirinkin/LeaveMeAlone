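; Player controller for LeaveMeAlone that handles pausing and the two end screens, game over and time over.
; Losing possession starts a one-second looping timer that counts down the spectation time, then triggers game over at zero.
; Each screen sets the pause flag, pauses the game, adds its widget and switches to UI-only input with a visible cursor.
; The pause input is ignored while already paused and stops the player's weapon fire first.
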(event Custom|TimeOver
  (Variables|Default|SetOnPause true)
  (Game|SetGamePaused true)
  (bind _returnvalue (UserInterface|CreateWidget "/Game/LeaveMeAlone/Widgets/UI/WBP_TimeOver.WBP_TimeOver_C"))
  (bind _output_get (Variables|Default|SetEndGameWidget _returnvalue))
  (UserInterface|Viewport|AddtoViewport _output_get 0)
  (Input|SetInputModeUIOnly self _output_get "DoNotLock" false)
  (Variables|Default|SetbShowMouseCursor true))

(event Custom|GameOver
  (Variables|Default|SetOnPause true)
  (Game|SetGamePaused true)
  (bind _returnvalue (UserInterface|CreateWidget "/Game/LeaveMeAlone/Widgets/UI/WBP_GameOver.WBP_GameOver_C"))
  (bind _output_get (Variables|Default|SetGameOverWidget _returnvalue))
  (UserInterface|Viewport|AddtoViewport _output_get 0)
  (Input|SetInputModeUIOnly self _output_get "DoNotLock" false)
  (Variables|Default|SetbShowMouseCursor true))

(event Custom|DecreaseTime
  (bind _output_get (Variables|Default|SetSpectationTime (- (Variables|Default|GetSpectationTime) 1)))
  (if (== _output_get 0)
    (Utilities|Time|ClearandInvalidateTimerbyHandle (Variables|Default|GetTimerHandler))
    (CallFunction|GameOver)))

(event EventBeginPlay)

(event EventTick
  (params (DeltaSeconds :type Float%20%28single-precision%29)))

(event EventUnPossess
  (params (UnpossessedPawn :type Pawn%20Object%20Reference))
  (bind _returnvalue (Utilities|Time|SetTimerbyEvent (delegate Custom|DecreaseTime) 1.0 true))
  (Variables|Default|SetTimerHandler _returnvalue))

(event Input|ActionEvents|InputActionPause
  (params (Key :type Key%20Structure :default "None"))
  (:Pressed
    (if (not (Variables|Default|GetOnPause))
      (Variables|Default|SetOnPause true)
      (bind _asch_player (Utilities|Casting|CastToCH_Player (Game|GetPlayerCharacter 0)))
      (Class|LMAWeaponComponent|StopFire (Variables|/Script/LeaveMeAlone.LMADefaultCharacter|GetWeaponComponent _asch_player))
      (Game|SetGamePaused true)
      (bind _returnvalue (UserInterface|CreateWidget "/Game/LeaveMeAlone/Widgets/UI/WBP_Pause.WBP_Pause_C"))
      (bind _output_get (Variables|Default|SetPauseWidget _returnvalue))
      (UserInterface|Viewport|AddtoViewport _output_get 0)
      (Input|SetInputModeUIOnly self _output_get "DoNotLock" false)
      (Variables|Default|SetbShowMouseCursor true))))

(fn ConstructionScript)