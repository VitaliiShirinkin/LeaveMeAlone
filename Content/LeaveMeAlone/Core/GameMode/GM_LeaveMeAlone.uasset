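; GM_LeaveMeAlone is the game mode that runs the match countdown.
; On BeginPlay it starts a looping one-second timer that decrements GameTime.
; When GameTime reaches zero it clears the timer and calls TimeOver on the first player controller, PC_LeaveMeAlone.
; If that cast fails, it opens the menu level instead.
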(event Custom|DecreaseTime
  (bind _output_get (Variables|Default|SetGameTime (- (Variables|Default|GetGameTime) 1)))
  (if (== _output_get 0)
    (Utilities|Time|ClearandInvalidateTimerbyHandle (Variables|Default|GetTimerController))
    (bind _aspc_leave_me_alone (Utilities|Casting|CastToPC_LeaveMeAlone (Game|GetPlayerController 0))
      (:then
        (Default|TimeOver _aspc_leave_me_alone))
      (:CastFailed
        (Game|OpenLevel(byObjectReference) "/Game/LeaveMeAlone/Levels/MenuLevel.MenuLevel")))))

(event EventBeginPlay
  (bind _returnvalue (Utilities|Time|SetTimerbyEvent (delegate Custom|DecreaseTime) 1.0 true))
  (Variables|Default|SetTimerController _returnvalue))

(event EventTick
  (params (DeltaSeconds :type Float%20%28single-precision%29)))

(fn ConstructionScript)